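; Zombie enemy Blueprint with a montage attack and physics-driven upper-body motion.
; BeginPlay simulates bodies from spine_02 down the bone chain with Physical Animation; BP_TraceGun capsule overlaps set full blend, then timers and a FlipFlop toggle Tick-driven blend reduction.
; Attack's montage notify sphere-overlaps player characters to apply damage, drawing a debug sphere, and montage end calls OnAttackEnd.
; Per-limb hit animations and PawnSensing blackboard logic are left disconnected.
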(event `self.ReceiveBeginPlay`
  ;[1 1 1] PhysicalAnimation을 이용해 좀더 좀비스러움 표현
  (`PhysicalAnimationComponent.SetSkeletalMeshComponent` (`self.PhysicalAnimation`) (`self.Mesh`))
  (`PhysicalAnimationComponent.ApplyPhysicalAnimationSettingsBelow` (`self.PhysicalAnimation`) "spine_02" (make `PhysicalAnimationData` false 500.0 100.0 500.0 100.0) true)
  (`SkeletalMeshComponent.SetAllBodiesBelowSimulatePhysics` (`self.Mesh`) "spine_02" true true))

(event `self.RightLeg.OnComponentHit`
  (params (HitComponent :type "PrimitiveComponent Object Reference") (OtherActor :type "Actor Object Reference") (OtherComp :type "PrimitiveComponent Object Reference") (NormalImpulse :type "Vector Structure") (Hit :type "HitResult Structure (by ref)"))
  ;[1 1 1] 부위별 콜라이더 충돌 시 피격 모션
)

(event `self.LeftLeg.OnComponentHit`
  (params (HitComponent :type "PrimitiveComponent Object Reference") (OtherActor :type "Actor Object Reference") (OtherComp :type "PrimitiveComponent Object Reference") (NormalImpulse :type "Vector Structure") (Hit :type "HitResult Structure (by ref)"))
  ;[1 1 1] 부위별 콜라이더 충돌 시 피격 모션
)

(event `self.RightHand.OnComponentHit`
  (params (HitComponent :type "PrimitiveComponent Object Reference") (OtherActor :type "Actor Object Reference") (OtherComp :type "PrimitiveComponent Object Reference") (NormalImpulse :type "Vector Structure") (Hit :type "HitResult Structure (by ref)"))
  ;[1 1 1] 부위별 콜라이더 충돌 시 피격 모션
)

(event `self.PawnSensing.OnSeePawn`
  (params (Pawn :type "Pawn Object Reference"))
  ;[1 1 1] 플레이어를 보면 쫒아옴(근데 안씀)
)

(event `self.LeftHand.OnComponentHit`
  (params (HitComponent :type "PrimitiveComponent Object Reference") (OtherActor :type "Actor Object Reference") (OtherComp :type "PrimitiveComponent Object Reference") (NormalImpulse :type "Vector Structure") (Hit :type "HitResult Structure (by ref)"))
  ;[1 1 1] 부위별 콜라이더 충돌 시 피격 모션
)

(event `self.Spine.OnComponentHit`
  (params (HitComponent :type "PrimitiveComponent Object Reference") (OtherActor :type "Actor Object Reference") (OtherComp :type "PrimitiveComponent Object Reference") (NormalImpulse :type "Vector Structure") (Hit :type "HitResult Structure (by ref)"))
  ;[1 1 1] 부위별 콜라이더 충돌 시 피격 모션
)

(event `Attack`
  (bind _returnvalue (`SceneComponent.K2_GetComponentLocation` (`self.AttackSphere`)))
  ;[1 1 1] 공격 & 공격 모션
  (`|PlayMontage` (`self.Mesh`) "/Game/CustomContents/Monster/WaveZombie/AM_WaveZombieAttack.AM_WaveZombieAttack"
    (:`OnCompleted`
      (`self.OnAttackEnd` :!label _label))
    (:`OnInterrupted`
      (goto _label))
    (:`OnNotifyBegin`
      (bind _outactors (`KismetSystemLibrary.SphereOverlapActors` _returnvalue (`self.AttackSphereRadius`) (`|MakeArray` "ObjectTypeQuery3" :!type "EObjectTypeQuery Enum") "/Game/ThirdPerson/Blueprints/BP_ThirdPersonCharacter.BP_ThirdPersonCharacter_C" (`|MakeArray` self :!type "Actor Object Reference")))
      (`KismetSystemLibrary.DrawDebugSphere` _returnvalue (`self.AttackSphereRadius`) 12 (struct :`R` 1.0 :`A` 1.0) (`self.SphereDuration`))
      (for _array_element _outactors
        (`GameplayStatics.ApplyDamage` _array_element (`self.AttackDamage`) (`self.GetController`) self "/Script/Engine.DamageType")))))

(event `self.Head.OnComponentHit`
  (params (HitComponent :type "PrimitiveComponent Object Reference") (OtherActor :type "Actor Object Reference") (OtherComp :type "PrimitiveComponent Object Reference") (NormalImpulse :type "Vector Structure") (Hit :type "HitResult Structure (by ref)"))
  ;[1 1 1] 부위별 콜라이더 충돌 시 피격 모션
)

(event `self.CapsuleComponent.OnComponentBeginOverlap`
  (params (OverlappedComponent :type "PrimitiveComponent Object Reference") (OtherActor :type "Actor Object Reference") (OtherComp :type "PrimitiveComponent Object Reference") (OtherBodyIndex :type Integer) (bFromSweep :type Boolean) (SweepResult :type "HitResult Structure (by ref)"))
  ;[1 1 1] Physical로 이용해 충돌시 부위판정(미완)
  (cast `/Game/CustomContents/Gun/BP_TraceGun` OtherActor)
  (`SkeletalMeshComponent.SetAllBodiesBelowPhysicsBlendWeight` (`self.Mesh`) "spine_02" 1.0 false true)
  (`KismetSystemLibrary.K2_SetTimer` null "PATrigger" 0.2))

(event `self.ReceiveTick`
  (params (DeltaSeconds :type "Float (single-precision)"))
  ;[1 1 1] Physical로 이용해 충돌시 부위판정(미완)
  (if (`self.DisablePA`)
    (`self.DisablePhysicalAnimation`)
    (`/Engine/EditorBlueprintResources/StandardMacros.DoOnce` false :!label _label_2
      (:`Completed`
        (`KismetSystemLibrary.K2_SetTimer` null "PATrigger" 0.2)))))

(event `PATrigger`
  ;[1 1 1] Physical로 이용해 충돌시 부위판정(미완)
  (`/Engine/EditorBlueprintResources/StandardMacros.FlipFlop`
    (:`A`
      (set `self.DisablePA` true)
      (goto _label_2 :!via `Reset`))
    (:`B`
      (set `self.DisablePA` false)
      (goto _label_2 :!via `Reset`))))

(event `DisablePhysicalAnimation`
  ;[1 1 1] Physical로 이용해 충돌시 부위판정(미완)
  (`SkeletalMeshComponent.SetAllBodiesBelowPhysicsBlendWeight` (`self.Mesh`) "spine_02" (`KismetMathLibrary.FInterpTo` 1.0 0.0 (`GameplayStatics.GetWorldDeltaSeconds`) 10.0) false true))

(fn `UserConstructionScript`)